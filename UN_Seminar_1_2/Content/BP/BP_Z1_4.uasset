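; BP_Z1_4 is an actor that grows as the player approaches and shrinks as they move away.
; Every tick it casts the player character to BP_ThirdPersonCharacter and measures the distance to it.
; It maps that distance linearly to a clamped uniform scale, so it is largest up close and settles to normal size at range.
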(event `self.ReceiveTick`
  (params (DeltaSeconds :type "Float (single-precision)"))
  (bind _asbp_third_person_character (cast `/Game/ThirdPerson/Blueprints/BP_ThirdPersonCharacter` (`GameplayStatics.GetPlayerCharacter` 0)))
  (`self.SetActorScale3D` (`KismetMathLibrary.Conv_DoubleToVector` (`KismetMathLibrary.FClamp` (- 6.0 (/ (`KismetMathLibrary.VSize` (- (`self.K2_GetActorLocation` _asbp_third_person_character) (`self.K2_GetActorLocation`))) 200.0)) 1.0 5.0))))

(fn `UserConstructionScript`)